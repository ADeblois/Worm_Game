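; Breakable branch Blueprint that reacts to hits from SilkShot.
; A box overlap casts the other actor to SilkShot, prints a debug string and calls BranchBreak, which applies fixed damage to the branch itself, with a Destructible component as its mesh.
; The construction script sizes the hit box and sets the destructible mesh and material from variables, leaving an unconnected SetStaticMesh node.
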(event OnComponentBeginOverlap(Box)
  (params (OverlappedComponent :type Primitive%20Component%20Object%20Reference) (OtherActor :type Actor%20Object%20Reference) (OtherComp :type Primitive%20Component%20Object%20Reference) (OtherBodyIndex :type Integer) (bFromSweep :type Boolean) (SweepResult :type Hit%20Result%20Structure%20%28by%20ref%29))
  (Utilities|Casting|CastToSilkShot OtherActor)
  (Development|PrintString "branch was hit")
  (CallFunction|BranchBreak))

(event Custom|Branch%20break
  (Game|Damage|ApplyDamage self 5.0 0 0))

(fn ConstructionScript
  (bind _destructible (Variables|Default|GetDestructible))
  (Components|Box|SetBoxExtent (Variables|Default|GetBox) (Variables|Default|GetHB%20extent) true)
  (if (!= _destructible 0)
    (Class|DestructibleComponent|SetDestructibleMesh _destructible (Variables|Default|GetdestroyableMesh))
    (Rendering|Material|SetMaterial (Variables|Default|GetDestructible) 0 (Variables|Default|GetMat))))