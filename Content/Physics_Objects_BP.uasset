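; Configurable physics prop actor whose mesh, material, mass and collision are exposed as variables.
; The construction script assigns the chosen static mesh and material when a mesh is set.
; BeginPlay applies mass scale, center-of-mass offset and collision type to the mesh and sizes the overlap sphere.
; Any actor overlap plays a 2D hit sound and spawns a hit particle emitter.
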(event EventBeginPlay
  (Class|PrimitiveComponent|SetMassScale (Variables|Default|GetSM) "None" (Variables|Physics|GetMass_SM))
  (Class|PrimitiveComponent|SetCenterOfMass (Variables|Default|GetSM) (Variables|Physics|GetCenter%20of%20Mass) "None")
  (Collision|SetCollisionEnabled (Variables|Default|GetSM) (Variables|Physics|GetCollision%20Type))
  (Components|Sphere|SetSphereRadius (Variables|Default|GetSphere) (Variables|Interaction|GetSphere%20Radius) true))

(event Collision|EventActorBeginOverlap
  (params (OtherActor :type Actor%20Object%20Reference))
  (Audio|PlaySound2D (Variables|Interaction|GetSound%20on%20Hit))
  (Effects|SpawnEmitteratLocation (Variables|Interaction|GetEmitter%20on%20hit) "0, 0, 0"))

(event EventTick
  (params (DeltaSeconds :type Float%20%28single-precision%29)))

(fn ConstructionScript
  (bind _static_mesh (Variables|Object|GetStatic%20Mesh))
  (bind _sm (Variables|Default|GetSM))
  (if (!= _static_mesh 0)
    (Components|StaticMesh|SetStaticMesh _sm _static_mesh)
    (Rendering|Material|SetMaterial _sm 0 (Variables|Object|GetMaterial))))