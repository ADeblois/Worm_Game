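; ToSequencer_BP is a box trigger actor that starts a sequencer cinematic when any actor other than the player character overlaps it.
; On overlap it plays a 2D sound, spawns a particle emitter, then waits a configurable delay before playing SequencerEvent.
; It then destroys its billboard and box components, with debug prints marking the collision and cleanup.
; The construction script sizes the box from the BoxExtent variable.
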(event EventBeginPlay)

(event Collision|EventActorBeginOverlap
  (params (OtherActor :type Actor%20Object%20Reference))
  (if (not (== OtherActor (Game|GetPlayerCharacter 0)))
    (Audio|PlaySound2D (Variables|Collision|GetSound%20on%20Hit))
    (Effects|SpawnEmitteratLocation (Variables|Collision|GetEmitter%20on%20Hit) "0, 0, 0")
    (Development|PrintString "I have collided!")
    (Utilities|FlowControl|Delay (Variables|Cinematics|GetDelay%20before%20Cinematic))
    (Audio|Components|Audio|Play (Variables|Cinematics|GetSequencer%20Event))
    (Components|DestroyComponent (Variables|Default|GetBillboard))
    (Development|PrintString "Goodbye!")))

(event EventTick
  (params (DeltaSeconds :type Float%20%28single-precision%29)))

(fn ConstructionScript
  (Components|Box|SetBoxExtent (Variables|Default|GetBox) (Variables|Default|GetBox%20Extent) true))