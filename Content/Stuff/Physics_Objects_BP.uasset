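; Configurable physics prop Blueprint whose mesh, material, mass, center of mass and collision type come from variables.
; The Construction Script applies the static mesh and material, while BeginPlay sets mass properties, collision mode and the Sphere component's radius.
; Mesh hits spawn an emitter with no location supplied and play an acorn sound at the mesh, followed by a Delay that leads nowhere.
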(event OnComponentHit(SM)
  (params (HitComponent :type Primitive%20Component%20Object%20Reference) (OtherActor :type Actor%20Object%20Reference) (OtherComp :type Primitive%20Component%20Object%20Reference) (NormalImpulse :type Vector :default "0, 0, 0") (Hit :type Hit%20Result%20Structure%20%28by%20ref%29))
  (Effects|SpawnEmitteratLocation (Variables|Interaction|GetEmitter%20on%20hit) "0, 0, 0")
  (Audio|PlaySoundatLocation "/Game/Sounds/Acorn_Cue.Acorn_Cue" (Transformation|GetWorldLocation (Variables|Default|GetSM)))
  (Utilities|FlowControl|Delay 2.0))

(event EventBeginPlay
  (Class|PrimitiveComponent|SetMassScale (Variables|Default|GetSM) "None" (Variables|Physics|GetMass_SM))
  (Class|PrimitiveComponent|SetCenterOfMass (Variables|Default|GetSM) (Variables|Physics|GetCenter%20of%20Mass) "None")
  (Collision|SetCollisionEnabled (Variables|Default|GetSM) (Variables|Physics|GetCollision%20Type))
  (Components|Sphere|SetSphereRadius (Variables|Default|GetSphere) (Variables|Interaction|GetSphere%20Radius) true))

(event Collision|EventActorBeginOverlap
  (params (OtherActor :type Actor%20Object%20Reference)))

(event EventTick
  (params (DeltaSeconds :type Float%20%28single-precision%29)))

(fn ConstructionScript
  (bind _static_mesh (Variables|Object|GetStatic%20Mesh))
  (bind _sm (Variables|Default|GetSM))
  (if (!= _static_mesh 0)
    (Components|StaticMesh|SetStaticMesh _sm _static_mesh)
    (Rendering|Material|SetMaterial _sm 0 (Variables|Object|GetMaterial))))