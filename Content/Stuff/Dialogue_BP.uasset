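; Dialogue trigger that shows text bubble planes when something overlaps its box, tied to an item retrieval objective.
; Overlap shows the first bubble, and an input event advances to the second, then hides both.
; Once Item_Retrieved_BP's score reaches one, overlap shows a completion bubble, then after a delay a final bubble, and sets Complete.
; The construction script applies configurable box extent, mesh and materials, assigning both final materials to the third plane.
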(event OnComponentEndOverlap(Box)
  (params (OverlappedComponent :type Primitive%20Component%20Object%20Reference) (OtherActor :type Actor%20Object%20Reference) (OtherComp :type Primitive%20Component%20Object%20Reference) (OtherBodyIndex :type Integer))
  ;[1 1 1] When player leaves overlap, hide all text boxes
  (Variables|Default|SetOverlapped false)
  (Development|SetHiddeninGame (Variables|Default|GetHow-To_Plane) true false)
  (Development|SetHiddeninGame (Variables|Default|GetHow-To_Plane_2) true false)
  (Variables|Default|SetTotal%20Key%20Presses 0))

(event OnComponentBeginOverlap(Box)
  (params (OverlappedComponent :type Primitive%20Component%20Object%20Reference) (OtherActor :type Actor%20Object%20Reference) (OtherComp :type Primitive%20Component%20Object%20Reference) (OtherBodyIndex :type Integer) (bFromSweep :type Boolean) (SweepResult :type Hit%20Result%20Structure%20%28by%20ref%29))
  ;[1 1 1] On overlap, set overlap to true. Get all actors from item retrieved bp. If item has been picked up, show final text bubble. If not, unhide first text box
  (if (Variables|Default|GetComplete)
    (Development|SetHiddeninGame (Variables|Default|GetHow-To_Plane_4) false false)
    (else
      (Variables|Default|SetOverlapped true)
      (bind _outactors (Actor|GetAllActorsOfClass "/Game/Stuff/Item_Retrieved_BP.Item_Retrieved_BP_C"))
      (if (>= (Variables|/Game/Stuff/Item_Retrieved_BP.Item_Retrieved_BP_C|GetScore_Item_Retrieved (Utilities|Array|Get(acopy) _outactors)) 1.0)
        (Development|SetHiddeninGame (Variables|Default|GetHow-To_Plane_3) false false)
        (Variables|Default|SetTotal%20Key%20Presses 0)
        (Utilities|FlowControl|Delay 3.0)
        (Development|SetHiddeninGame (Variables|Default|GetHow-To_Plane_3) true false)
        (Development|SetHiddeninGame (Variables|Default|GetHow-To_Plane_4) false false)
        (Variables|Default|SetComplete true)
        (else
          (Development|SetHiddeninGame (Variables|Default|GetHow-To_Plane) false false))))))

(event Custom|External_input
  ;[1 1 1] If G is released after the key pressed number is set,  and is overlapping, hide all
  (if (Variables|Default|GetComplete)
    (Development|SetHiddeninGame (Variables|Default|GetHow-To_Plane_4) false false)
    (elif (>= (+ (Variables|Default|GetTotal%20Key%20Presses) 1) 2)
      (Development|SetHiddeninGame (Variables|Default|GetHow-To_Plane) true false :!label _label)
      (Development|SetHiddeninGame (Variables|Default|GetHow-To_Plane_2) true false)
      (Variables|Default|SetTotal%20Key%20Presses 0)
      (else
        (Variables|Default|SetTotal%20Key%20Presses (+ (Variables|Default|GetTotal%20Key%20Presses) 1))
        (switch int (Variables|Default|GetTotal%20Key%20Presses)
          (:0
            _)
          (:1
            _)
          (:2
            (goto _label)))
        (Development|SetHiddeninGame (Variables|Default|GetHow-To_Plane) true false)
        (Development|SetHiddeninGame (Variables|Default|GetHow-To_Plane_2) false false)))))

(event EventBeginPlay
  ;[1 1 1] Event Begin, Hide both text boxes. MAKE SURE INPUT IS ENABLED
  (Development|SetHiddeninGame (Variables|Default|GetHow-To_Plane) true false)
  (Development|SetHiddeninGame (Variables|Default|GetHow-To_Plane_2) true false)
  (Development|SetHiddeninGame (Variables|Default|GetHow-To_Plane_3) true false)
  (Input|EnableInput (Game|GetPlayerController 0)))

(fn ConstructionScript
  (bind _static_mesh (Variables|Default|GetStatic%20Mesh))
  ;[1 1 1] Set Box Extent
  (Components|Box|SetBoxExtent (Variables|Default|GetBox) (Variables|Default|GetBox%20Extent) true)
  ;[1 1 1] Change Static Mesh
  (if (!= _static_mesh 0)
    (Components|StaticMesh|SetStaticMesh (Variables|Default|GetHow-To_Plane) _static_mesh)
    (Components|StaticMesh|SetStaticMesh (Variables|Default|GetHow-To_Plane_2) _static_mesh)
    (Components|StaticMesh|SetStaticMesh (Variables|Default|GetHow-To_Plane_3) _static_mesh)
    ;[1 1 1] Change Material
    (Rendering|Material|SetMaterial (Variables|Default|GetHow-To_Plane) 0 (Variables|Dialogue|GetFirst%20Text%20Bubble))
    (Rendering|Material|SetMaterial (Variables|Default|GetHow-To_Plane_2) 0 (Variables|Dialogue|GetSecond%20Text%20Bubble))
    (Rendering|Material|SetMaterial (Variables|Default|GetHow-To_Plane_3) 0 (Variables|Dialogue|GetFinal%20Text%20Bubble))
    (Rendering|Material|SetMaterial (Variables|Default|GetHow-To_Plane_3) 0 (Variables|Dialogue|GetFinal%20Text%20Bubble%202))))