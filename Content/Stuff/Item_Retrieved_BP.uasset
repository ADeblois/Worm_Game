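; Retrievable item actor that the Pete_Test character collects by overlapping its box.
; The construction script applies a configurable mesh, material and box extent when the mesh variable passes its check.
; On overlap, it adds one to its own ScoreItemRetrieved variable, then destroys its billboard, box and cube components rather than the actor itself.
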(event OnComponentBeginOverlap(Box)
  (params (OverlappedComponent :type Primitive%20Component%20Object%20Reference) (OtherActor :type Actor%20Object%20Reference) (OtherComp :type Primitive%20Component%20Object%20Reference) (OtherBodyIndex :type Integer) (bFromSweep :type Boolean) (SweepResult :type Hit%20Result%20Structure%20%28by%20ref%29))
  ;[1 1 1] When overlapped run item retrieve score and destroy actor
  (Utilities|Casting|CastToPete_Test OtherActor)
  (CallFunction|ItemRetrievedScore)
  (Components|DestroyComponent (Variables|Default|GetBillboard)))

(fn ConstructionScript
  (bind _static_mesh (Variables|Default|GetStatic%20Mesh))
  (bind _cube (Variables|Default|GetCube))
  ;[1 1 1] Set Mesh Variable and Material Variable
  (if (!= _static_mesh 0)
    (Components|StaticMesh|SetStaticMesh _cube _static_mesh)
    (Rendering|Material|SetMaterial _cube 0 (Variables|Mesh|GetMaterial))
    ;[1 1 1] Set Box Extent
    (Components|Box|SetBoxExtent (Variables|Default|GetBox) (Variables|Default|GetBox%20Extent) true)))

(fn ItemRetrievedScore
  ;[1 1 1] When run, add 1 to Score Item Retrieved and set new score
  (Variables|Default|SetScore_Item_Retrieved (+ (Variables|Default|GetScore_Item_Retrieved) 1.0)))